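; BP_ConanWorldComposition supplies the world positions that streaming is based on, through its GetStreamingPositions function.
; It uses the location of player controller 0's controlled pawn, falling back to the controller's InitialPlayerStart when no pawn is valid.
; With neither available, it adds every actor tagged for character creation.
; A Sequence node returns the Positions array after this lookup, even if the controller is missing or the cast fails.
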(fn GetStreamingPositions
  (bind _returnvalue (Game|GetPlayerController 0))
  (bind _positions (LocalVariables|GetPositions))
  (Utilities|FlowControl|Sequence
    (:then_0
      (Utilities|IsValid _returnvalue
        (:Is%20Valid
          (bind _asconan_player_controller (Utilities|Casting|CastToConanPlayerController _returnvalue))
          (LocalVariables|SetPlayerController _asconan_player_controller)
          (Utilities|IsValid (Pawn|GetControlledPawn _asconan_player_controller)
            (:Is%20Valid
              (Utilities|Array|Add _positions (Transformation|GetActorLocation (Pawn|GetControlledPawn _asconan_player_controller))))
            (:Is%20Not%20Valid
              (Utilities|IsValid (Variables|/Script/ConanSandbox.ConanPlayerController|GetInitialPlayerStart _asconan_player_controller)
                (:Is%20Valid
                  (Utilities|Array|Add _positions (Transformation|GetActorLocation (Variables|/Script/ConanSandbox.ConanPlayerController|GetInitialPlayerStart _asconan_player_controller))))
                (:Is%20Not%20Valid
                  (bind _outactors (Actor|GetAllActorswithTag (Variables|Default|GetCharacterCreationTag)))
                  (for _array_element _outactors
                    (Utilities|Array|Add (LocalVariables|GetPositions) (Transformation|GetActorLocation _array_element))))))))))
    (:then_1
      (return (LocalVariables|GetPositions)))))