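; Hanging brazier prop Blueprint that lights and extinguishes itself automatically with the time of day.
; Every Tick it reads the hour from TimeManager and counts evening through early morning as lit hours.
; It then toggles the small fire particle, its audio and the point light together, using the particle's active state as a guard so changes only happen on transitions.
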(event EventTick
  (params (DeltaSeconds :type Float%20%28single-precision%29))
  (bind _p_fire_small (Variables|Default|GetP_Fire_Small))
  (bind _returnvalue (Components|Activation|IsActive _p_fire_small))
  (bind _returnvalue_2 (Class|ConanTimeOfDayManager|GetTimeOfDay (Variables|Default|Gettime%20manager)))
  (Utilities|Or+Branch (>= _returnvalue_2 17.0) (<= _returnvalue_2 6.0)
    (:True
      (if (not _returnvalue)
        (Components|Activation|Activate (Variables|Default|GetP_Fire_Small) false)
        (Components|Activation|Activate (Variables|Default|GetConanAudio1) false)
        (Rendering|SetVisibility (Variables|Default|GetPointLight1) true false)))
    (:False
      (if _returnvalue
        (Components|Activation|Deactivate (Variables|Default|GetP_Fire_Small))
        (Components|Activation|Deactivate (Variables|Default|GetConanAudio1))
        (Rendering|SetVisibility (Variables|Default|GetPointLight1) false false)))))

(fn ConstructionScript)