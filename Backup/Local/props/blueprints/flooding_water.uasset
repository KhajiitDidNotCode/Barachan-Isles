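; Flooding water actor that rises and falls like a tide according to the time of day.
; Each Tick it reads TimeManager's time and, within set one-hour windows, nudges its Z position up or down, four windows each way.
; Movement is a fixed step per frame without delta-time scaling, so the water height reached depends on frame rate.
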(event EventTick
  (params (DeltaSeconds :type Float%20%28single-precision%29))
  (bind _returnvalue (Transformation|GetActorLocation))
  (bind (_x _y _z) (Math|Vector|BreakVector _returnvalue))
  (bind _returnvalue_2 (Class|ConanTimeOfDayManager|GetTimeOfDay (Variables|Default|Gettime%20manager)))
  (if (Math|Conversions|ToBoolean(Integer) (.ReturnValue (Math|Float|Division(WholeandRemainder) _returnvalue_2 2.0)))
    (if (Math|Boolean|ORBoolean (and (> _returnvalue_2 2.0) (< _returnvalue_2 3.0)) (and (> _returnvalue_2 1e+01) (< _returnvalue_2 11.0)) (and (> _returnvalue_2 14.0) (< _returnvalue_2 15.0)) (and (> _returnvalue_2 22.0) (< _returnvalue_2 23.0)))
      (Transformation|SetActorLocation (Math|Vector|MakeVector _x _y (+ _z 0.05)) false false)
      (elif (Math|Boolean|ORBoolean (and (> _returnvalue_2 4.0) (< _returnvalue_2 5.0)) (and (> _returnvalue_2 8.0) (< _returnvalue_2 9.0)) (and (> _returnvalue_2 16.0) (< _returnvalue_2 17.0)) (and (> _returnvalue_2 2e+01) (< _returnvalue_2 21.0)))
        (Transformation|SetActorLocation (Math|Vector|MakeVector _x _y (+ _z -0.05)) false false)))))

(fn ConstructionScript)